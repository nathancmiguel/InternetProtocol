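; BPC_WebsocketClient is a WebSocket client Blueprint laid out as an unwired template of the client API, so none of it runs.
; Its event graph holds empty handlers for connection, handshake, message, ping, pong, close, error and send-completion events.
; Loose, unexecuted nodes show event binding, connecting, text and buffer writes, closing, and rooting against garbage collection.
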(event Custom|MessageSent
  (params (ErrorCode :type Error%20Code%20Structure%20%28by%20ref%29) (BytesSent :type Integer))
  ;[0 0 0] Websocket
)

(event Custom|BufferSent
  (params (ErrorCode :type Error%20Code%20Structure%20%28by%20ref%29) (BytesSent :type Integer))
  ;[0 0 0] Websocket
)

(event Custom|PingSent
  (params (ErrorCode :type Error%20Code%20Structure%20%28by%20ref%29) (BytesSent :type Integer))
  ;[0 0 0] Websocket
)

(event Custom|PongEvent
  (params (ErrorCode :type Error%20Code%20Structure%20%28by%20ref%29) (BytesSent :type Integer))
  ;[0 0 0] Websocket
)

(event Custom|Connected
  (params (Handshake :type Http%20Request%20Structure%20%28by%20ref%29))
  ;[0 0 0] Events
)

(event Custom|Message
  (params (Buffer :type Array%20of%20Bytes) (bIsBinary :type Boolean))
  ;[0 0 0] Events
)

(event Custom|UnexpectedHandshake
  (params (Handshake :type Http%20Request%20Structure%20%28by%20ref%29))
  ;[0 0 0] Events
)

(event Custom|OnPing_Event
  ;[0 0 0] Events
)

(event Custom|OnPong_Event
  ;[0 0 0] Events
)

(event Custom|OnClose_Event
  (params (Code :type Integer) (Reason :type String))
  ;[0 0 0] Events
)

(event Custom|OnError_Event
  (params (ErrorCode :type Error%20Code%20Structure%20%28by%20ref%29))
  ;[0 0 0] Events
)