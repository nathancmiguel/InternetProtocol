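; BPC_UDPClient is a reference scaffold for a UDP client's Blueprint API, with no working game logic.
; It lays out nodes for connecting, closing, sending messages or buffers, socket queries, and rooting against garbage collection.
; Handlers for connection, received message, close, error and send completion are empty stubs.
; None of the calls or event bindings are wired to an execution path, so nothing runs.
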(event Custom|Error
  (params (ErrorCode :type Error%20Code%20Structure%20%28by%20ref%29))
  ;[0 0 0] Events
)

(event Custom|OnMessageSent
  (params (ErrorCode :type Error%20Code%20Structure%20%28by%20ref%29) (BytesSent :type Integer))
  ;[0 0 0] UDP
)

(event Custom|OnBufferSent
  (params (ErrorCode :type Error%20Code%20Structure%20%28by%20ref%29) (BytesSent :type Integer))
  ;[0 0 0] UDP
)

(event Custom|Connected
  ;[0 0 0] Events
)

(event Custom|Message
  (params (Buffer :type Array%20of%20Bytes) (BytesRecv :type Integer))
  ;[0 0 0] Events
)

(event Custom|OnClose_Event
  ;[0 0 0] Events
)