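; BPC_HttpServer is an HTTP server Blueprint that lays out the server API as an unwired template.
; Empty handler events are bound to route nodes for each HTTP method plus a catch-all, alongside empty close and error events.
; Loose nodes cover opening, closing, connection settings, status queries and rooting against garbage collection.
; No node is connected to an execution entry, so the graph does nothing as it stands.
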(event Custom|AllMethod
  (params (Request :type Http%20Request%20Structure%20%28by%20ref%29) (Response :type Http%20Remote%20Object%20Reference))
  ;[0 0 0] HTTP
)

(event Custom|GetMethod
  (params (Request :type Http%20Request%20Structure%20%28by%20ref%29) (Response :type Http%20Remote%20Object%20Reference))
  ;[0 0 0] HTTP
)

(event Custom|PostMethod
  (params (Request :type Http%20Request%20Structure%20%28by%20ref%29) (Response :type Http%20Remote%20Object%20Reference))
  ;[0 0 0] HTTP
)

(event Custom|PutMethod
  (params (Request :type Http%20Request%20Structure%20%28by%20ref%29) (Response :type Http%20Remote%20Object%20Reference))
  ;[0 0 0] HTTP
)

(event Custom|DelMethod
  (params (Request :type Http%20Request%20Structure%20%28by%20ref%29) (Response :type Http%20Remote%20Object%20Reference))
  ;[0 0 0] HTTP
)

(event Custom|HeadMethod
  (params (Request :type Http%20Request%20Structure%20%28by%20ref%29) (Response :type Http%20Remote%20Object%20Reference))
  ;[0 0 0] HTTP
)

(event Custom|OptionsMethod
  (params (Request :type Http%20Request%20Structure%20%28by%20ref%29) (Response :type Http%20Remote%20Object%20Reference))
  ;[0 0 0] HTTP
)

(event Custom|PatchMethod
  (params (Request :type Http%20Request%20Structure%20%28by%20ref%29) (Response :type Http%20Remote%20Object%20Reference))
  ;[0 0 0] HTTP
)

(event Custom|OnClose_Event
  ;[0 0 0] EVENTS
)

(event Custom|Error
  (params (ErrorCode :type Error%20Code%20Structure%20%28by%20ref%29))
  ;[0 0 0] EVENTS
)